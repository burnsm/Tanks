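; BP_MyHUD is a HUD class that draws the game's directions panel and win or loss screens.
; On each DrawHUD it shows the Directions texture near the top-right corner while MainMenuOn is set.
; A Won flag draws a centered YouWin image, otherwise a Loss flag draws a centered loss image.
; The flags are only read here, and all layout uses fixed pixel sizes and offsets from the screen size.
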(event `self.ReceiveDrawHUD`
  (params (SizeX :type Integer) (SizeY :type Integer))
  (if (`self.MainMenuOn`)
    (`self.DrawTexture` "/Game/Directions.Directions" (`KismetMathLibrary.Conv_IntToDouble` (- SizeX 250)) 40.0 206.0 145.0))
  (if (`self.won`)
    (`self.DrawTexture` "/Game/YouWin.YouWin" (`KismetMathLibrary.Conv_IntToDouble` (- (/ SizeX 2) 247)) (`KismetMathLibrary.Conv_IntToDouble` (- (/ SizeY 2) 118)) 495.0 236.0 0.0 0.0 1.0 1.0)
    (elif (`self.loss`)
      (`self.DrawTexture` "/Game/L.L" (`KismetMathLibrary.Conv_IntToDouble` (- (/ SizeX 2) 250)) (`KismetMathLibrary.Conv_IntToDouble` (- (/ SizeY 2) 250)) 500.0 500.0 0.0 0.0 1.0 1.0))))

(event `self.ReceiveBeginPlay`)

(event `self.ReceiveActorBeginOverlap`
  (params (OtherActor :type "Actor Object Reference")))

(fn `UserConstructionScript`)