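; Behavior Tree task that moves an AI-controlled Enemy pawn toward the actor in the Enemy blackboard key, then fires.
; It caches the EnemyController, runs AIMoveTo and, on success, passes Fire a negated pitch angle computed from height difference over horizontal distance.
; Both move success and move failure finish the task as failed; a failed cast stops without finishing it.
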(event `self.ReceiveExecute`
  (params (OwnerActor :type "Actor Object Reference"))
  (bind _returnvalue (`Controller.K2_GetPawn` (`self.AI_CON_Ref`)))
  (bind _returnvalue_2 (`BTFunctionLibrary.GetBlackboardValueAsActor` (`self.Enemy`)))
  (bind (_returnvalue_x _returnvalue_y _returnvalue_z) (`KismetMathLibrary.BreakVector` (`Actor.K2_GetActorLocation` _returnvalue)))
  (bind (_returnvalue_x_2 _returnvalue_y_2 _returnvalue_z_2) (`KismetMathLibrary.BreakVector` (`Actor.K2_GetActorLocation` _returnvalue_2)))
  (if (not (!= (`self.AI_CON_Ref`) null))
    (bind _asenemy_controller (cast `EnemyController` OwnerActor))
    (set `self.AI_CON_Ref` _asenemy_controller))
  (`|AIMoveTo` _returnvalue (0.0 0.0 0.0) _returnvalue_2 200.0
    (:`OnSuccess`
      (bind _asenemy (cast `Enemy` _returnvalue))
      (`Enemy.fire` _asenemy (- 0.0 (`KismetMathLibrary.DegAtan` (/ (- _returnvalue_z_2 _returnvalue_z) (`KismetMathLibrary.Sqrt` (+ (`KismetMathLibrary.Square` (- _returnvalue_y_2 _returnvalue_y)) (`KismetMathLibrary.Square` (- _returnvalue_x_2 _returnvalue_x)))))))))
    (:`OnFail`
      _))
  (`self.FinishExecute` false))