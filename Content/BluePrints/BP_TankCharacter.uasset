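; Tank character Blueprint that handles aiming and camera switching for the tank.
; Yaw input turns the Turret and SpringArm together, using a pitch-derived sine/cosine axis so the arm's local rotation compensates for its tilt.
; Pitch input tilts the SpringArm and rotates the Barrel on its local roll axis, scaled by a separate look speed.
; The C key flip-flops the active camera between Camera1 and Camera2.
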(event `self.ReceiveBeginPlay`)

(event `self.ReceiveActorBeginOverlap`
  (params (OtherActor :type "Actor Object Reference")))

(event `self.ReceiveTick`
  (params (DeltaSeconds :type "Float (single-precision)")))

(event `InputAxis|Yaw`
  (params (AxisValue :type "Float (single-precision)"))
  (bind _returnvalue_pitch (`KismetMathLibrary.BreakRotator` (`SceneComponent.GetSocketRotation` (`self.SpringArm`) "None")))
  (bind _returnvalue (* AxisValue (`self.Look Speed X`)))
  (`SceneComponent.K2_AddLocalRotation` (`self.SpringArm`) (`KismetMathLibrary.RotatorFromAxisAndAngle` (`KismetMathLibrary.MakeVector` (`KismetMathLibrary.DegSin` _returnvalue_pitch) 0.0 (`KismetMathLibrary.DegCos` _returnvalue_pitch)) _returnvalue) false)
  (`SceneComponent.K2_AddLocalRotation` (`self.turret`) (`KismetMathLibrary.MakeRotator` 0.0 _returnvalue) false))

(event `InputAxis|Pitch`
  (params (AxisValue :type "Float (single-precision)"))
  (bind _returnvalue (* AxisValue (`self.Look Speed Y`)))
  (bind _result (`/Engine/EditorBlueprintResources/StandardMacros.NegateFloat` _returnvalue)
    (:`  `
      (`SceneComponent.K2_AddLocalRotation` (`self.SpringArm`) (`KismetMathLibrary.MakeRotator` _result) false)
      (`SceneComponent.K2_AddLocalRotation` (`self.barrel`) (`KismetMathLibrary.MakeRotator` 0.0 0.0 _returnvalue) false))))

(event `Key|C`
  (:`Pressed`
    (`/Engine/EditorBlueprintResources/StandardMacros.FlipFlop`
      (:`A`
        (`ActorComponent.SetActive` (`self.Camera1`) false false)
        (`ActorComponent.SetActive` (`self.Camera2`) true false))
      (:`B`
        (`ActorComponent.SetActive` (`self.Camera2`) false false)
        (`ActorComponent.SetActive` (`self.Camera1`) true false)))))

(fn `UserConstructionScript`)